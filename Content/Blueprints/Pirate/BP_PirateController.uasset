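; BP_PirateController is a controller that lets the player click chests in the world with a visible mouse cursor.
; On BeginPlay it shows the cursor and sets Game and UI input with the mouse locked to the viewport.
; A left click runs a Visibility line trace from the deprojected mouse position, calls ChestClicked on any BP_Chest hit and prints a string.
; The trace still draws persistent debug lines.
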(event `self.ReceiveBeginPlay`
  (set `self.bShowMouseCursor` true)
  (`WidgetBlueprintLibrary.SetInputMode_GameAndUIEx` self null "LockAlways" false true))

(event `Key|LeftMouseButton`
  (params (Key :type "Key Structure"))
  (bind (_worldlocation _worlddirection) (`self.DeprojectMousePositionToWorld`))
  (:`Pressed`
    (bind _outhit (`KismetSystemLibrary.LineTraceSingle` :`Start` _worldlocation :`End` (+ _worldlocation (* _worlddirection 10000.0)) :`TraceChannel` "TraceTypeQuery1" :`DrawDebugType` "Persistent"))
    (bind _asbp_chest (cast `/Game/Blueprints/Chest/BP_Chest` (`.HitActor` (`GameplayStatics.BreakHitResult` _outhit))))
    (`/Game/Blueprints/Chest/BP_Chest.ChestClicked` _asbp_chest)
    (`KismetSystemLibrary.PrintString` "Hello")))

(fn `UserConstructionScript`)