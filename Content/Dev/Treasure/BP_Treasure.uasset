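; BP_Treasure is a treasure actor that takes its look from a context and plays a gem tap sound on interaction.
; It starts hidden with tick off until Initialize applies the context's mesh and material, then shows it and enables tick.
; A Debug flag makes it initialize itself on BeginPlay from its own TreasureContext.
; Interact only plays the sound, and Initialize prints the mesh name.
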(event `self.ReceiveBeginPlay`
  (`self.SetActorHiddenInGame` true)
  (`self.SetActorTickEnabled` false)
  (if (`self.Debug`)
    (`self.Initialize` (`self.TreasureContext`))))

(event `InteractableInterface.Interact`
  (params (Source :type "Object Object Reference"))
  (`/Game/Dev/Libraries/BPFL_Sound.PlaySound` (`self.Audio`) "/Game/Dev/Shelf/SC_GemTap.SC_GemTap"))

(fn `Initialize`
  (params (Context :type "TreasureContext Structure"))
  (bind (_mesh _material) (break `TreasureContext` Context))
  (bind _staticmesh (`self.StaticMesh`))
  (`KismetSystemLibrary.PrintString` (`KismetStringLibrary.Conv_ObjectToString` _mesh))
  (`StaticMeshComponent.SetStaticMesh` _staticmesh _mesh)
  (`PrimitiveComponent.SetMaterial` _staticmesh 0 _material)
  (`self.SetActorHiddenInGame` false)
  (`self.SetActorTickEnabled` true))

(fn `UserConstructionScript`)