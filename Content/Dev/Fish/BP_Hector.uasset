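; BP_Hector is a heckler that plays a random voice or sound clip whenever a fish is clicked in the pirate gacha game.
; It binds to the FishClicked dispatcher on BP_PirateGachaGameMode at BeginPlay, then sets IsHeckling and swaps the HecklingAudio sound on each broadcast.
; Tick polls the audio component and clears IsHeckling whenever nothing is playing, rather than binding a finished event.
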(event `self.ReceiveBeginPlay`
  (bind _asbp_pirate_gacha_game_mode (cast `/Game/Dev/Mode/BP_PirateGachaGameMode` (`GameplayStatics.GetGameMode`)))
  (add `/Game/Dev/Mode/BP_PirateGachaGameMode.ED_FishClicked` _asbp_pirate_gacha_game_mode (delegate `ED_FishClicked_Event`)))

(event `ED_FishClicked_Event`
  (bind _hecklingaudio (`self.HecklingAudio`))
  (set `self.IsHeckling` true)
  (`AudioComponent.SetSound` _hecklingaudio (`KismetArrayLibrary.Array_Random` (`|MakeArray` "/Game/Audio/voicelines/fishClick/fishClick_1-Audio.fishClick_1-Audio" "/Game/Audio/voicelines/fishClick/fishClick_10-Audio.fishClick_10-Audio" "/Game/Audio/voicelines/fishClick/fishClick_11-Audio.fishClick_11-Audio" "/Game/Audio/voicelines/fishClick/fishClick_12-Audio.fishClick_12-Audio" "/Game/Audio/voicelines/fishClick/fishClick_13-Audio.fishClick_13-Audio" "/Game/Audio/voicelines/fishClick/fishClick_14-Audio.fishClick_14-Audio" "/Game/Audio/voicelines/fishClick/fishClick_2-Audio.fishClick_2-Audio" "/Game/Audio/voicelines/fishClick/fishClick_3-Audio.fishClick_3-Audio" "/Game/Audio/voicelines/fishClick/fishClick_4-Audio.fishClick_4-Audio" "/Game/Audio/voicelines/fishClick/fishClick_5-Audio.fishClick_5-Audio" "/Game/Audio/voicelines/fishClick/fishClick_6-Audio.fishClick_6-Audio" "/Game/Audio/voicelines/fishClick/fishClick_7-Audio.fishClick_7-Audio" "/Game/Audio/voicelines/fishClick/fishClick_8-Audio.fishClick_8-Audio" "/Game/Audio/voicelines/fishClick/fishClick_9-Audio.fishClick_9-Audio" "/Game/Audio/voicelines/fishClick/fishClick_14-Audio.fishClick_14-Audio" :!type "SoundBase Object Reference")))
  (`AudioComponent.Play` _hecklingaudio 0.0))

(event `self.ReceiveTick`
  (params (DeltaSeconds :type "Float (single-precision)"))
  (if (not (`AudioComponent.IsPlaying` (`self.HecklingAudio`)))
    (`self.AudioDonePlaying`)))

(event `AudioDonePlaying`
  (set `self.IsHeckling` false))

(fn `UserConstructionScript`)