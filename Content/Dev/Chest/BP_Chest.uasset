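; Paid loot chest that opens when the interactor pays its cost, with a chance to spawn a random data-table treasure at a socket until it closes.
; STM_Chest owns the state, taking open, close and hover-shake requests and re-emitting changes through chest dispatchers.
; State changes drive ABP_Chest, whose animation-done events feed back to advance the state machine.
; A toggleable gold pile mesh follows the chest skeleton via leader pose.
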(event `self.StateMachine.OnStateMachineInitializedEvent`
  (params (Instance :type "SMInstance Object Reference"))
  ;[1 1 1] Initialize
  (bind _asstm_chest (cast `/Game/Dev/Chest/STM_Chest` Instance)
    (:`then`
      (set `self.STM_Chest` _asstm_chest)
      (bind _asabp_chest (cast `/Game/Dev/Chest/ABP_Chest` (`SkeletalMeshComponent.GetAnimInstance` (`self.SK_Chest`)))
        (:`then`
          (set `self.AnimationBlueprint` _asabp_chest)
          ;[1 1 1] Bind listeners
          ;;[1 1 1] Emits
          (add `/Game/Dev/Chest/STM_Chest.OnStateChange` (`self.STM_Chest`) (delegate `StateChange`))
          (add `/Game/Dev/Chest/STM_Chest.OnOpening` (`self.STM_Chest`) (delegate `Opening`))
          (add `/Game/Dev/Chest/STM_Chest.OnOpened` (`self.STM_Chest`) (delegate `Opened`))
          (add `/Game/Dev/Chest/STM_Chest.OnClosing` (`self.STM_Chest`) (delegate `Closing`))
          (add `/Game/Dev/Chest/STM_Chest.OnClosed` (`self.STM_Chest`) (delegate `Closed`))
          (add `/Game/Dev/Chest/STM_Chest.OnShaking` (`self.STM_Chest`) (delegate `Shaking`))
          ;;[1 1 1] Animation
          (add `self.OnStateChange` (delegate `NotifyAnimation`))
          (add `/Game/Dev/Chest/ABP_Chest.OnAnimationOpenChestDone` (`self.AnimationBlueprint`) (delegate `AnimationOpenDone`))
          (add `/Game/Dev/Chest/ABP_Chest.OnAnimationCloseChestDone` (`self.AnimationBlueprint`) (delegate `AnimationCloseDone`)))
        (:`CastFailed`
          (`KismetSystemLibrary.PrintString` "Fatal chest error, unable to locate animation blueprint."))))
    (:`CastFailed`
      (`KismetSystemLibrary.PrintString` "Fatal chest error, unable to locate state machine." true true (struct :`R` 1.0 :`B` 0.159335 :`A` 1.0) 10.0))))

(event `StateChange`
  (params (State :type "/Game/Dev/Chest/E_ChestState Enum" :default "NewEnumerator0"))
  ;[1 1 1] Bind listeners
  ;;[1 1 1] Emits
  (`self.OnStateChange` (`self.Context`) State))

(event `Opening`
  ;[1 1 1] Bind listeners
  ;;[1 1 1] Emits
  (`self.OnOpening` (`self.Context`)))

(event `Opened`
  ;[1 1 1] Bind listeners
  ;;[1 1 1] Emits
  (`self.OnOpened` (`self.Context`)))

(event `Closing`
  ;[1 1 1] Bind listeners
  ;;[1 1 1] Emits
  (`self.OnClosing` (`self.Context`)))

(event `Closed`
  ;[1 1 1] Bind listeners
  ;;[1 1 1] Emits
  (`self.OnClosed` (`self.Context`)))

(event `Shaking`
  ;[1 1 1] Bind listeners
  ;;[1 1 1] Emits
  (`self.OnShaking` (`self.Context`)))

(event `NotifyAnimation` :!signature `self.OnStateChange`
  (params (Context :type "ChestContext Structure") (State :type "/Game/Dev/Chest/E_ChestState Enum" :default "NewEnumerator0"))
  ;[1 1 1] Bind listeners
  ;;[1 1 1] Animation
  (`/Game/Dev/Chest/ABP_Chest.SendUpdateAnimationState` (`self.AnimationBlueprint`) State))

(event `AnimationOpenDone`
  ;[1 1 1] Bind listeners
  ;;[1 1 1] Animation
  (`/Game/Dev/Chest/STM_Chest.SendOpenDone` (`self.STM_Chest`)))

(event `AnimationCloseDone`
  ;[1 1 1] Bind listeners
  ;;[1 1 1] Animation
  (`/Game/Dev/Chest/STM_Chest.SendCloseDone` (`self.STM_Chest`)))

(event `InteractableInterface.Interact`
  (params (Source :type "Object Object Reference"))
  (bind (_treasure _success) (`self.GenerateTreasure` (`.Chance` (break `ChestContext` (`self.Context`)))))
  ;[1 1 1] Interact interface implementation
  (bind _state (`self.GetState`))
  (switch `/Game/Dev/Chest/E_ChestState` _state
    (:`NewEnumerator0`
      _)
    (:`NewEnumerator3`
      _))
  (bind _returnvalue (message `RequestPayInterface.RequestPay` Source self (`.Cost` (break `ChestContext` (`self.Context`)))))
  (if _returnvalue
    (`self.Open`)
    (if _success
      (bind _treasure_ref (`self.Spawn Treasure` _treasure))
      (add `self.OnClosed` (delegate `RemoveTreasureOnClose`)))))

(event `RemoveTreasureOnClose` :!signature `self.OnClosed`
  (params (Context :type "ChestContext Structure"))
  ;[1 1 1] Interact interface implementation
  (`self.K2_DestroyActor` (stale `InteractableInterface.Interact` _treasure_ref))
  (remove `self.OnClosed` (delegate `RemoveTreasureOnClose`)))

(event `HoverableInterface.Hover`
  (params (isHovering :type Boolean))
  (bind _stm_chest (`self.STM_Chest`))
  ;[1 1 1] Hover interface implementation
  (if isHovering
    (`/Game/Dev/Chest/STM_Chest.SendShakingStart` _stm_chest)
    (else
      (`/Game/Dev/Chest/STM_Chest.SendShakingStop` _stm_chest))))

(fn `Close`
  (`/Game/Dev/Chest/STM_Chest.SendClose` (`self.STM_Chest`)))

(fn `GenerateTreasure`
  (params (`Treasure Chance` :type "Float (double-precision)"))
  (returns (Treasure :type "TreasureContext Structure") (Success :type Boolean))
  (if (<= (`KismetMathLibrary.RandomFloat`) `Treasure Chance`)
    (bind _outrownames (`DataTableFunctionLibrary.GetDataTableRowNames` "/Game/Dev/Treasure/DT_TreasureContext.DT_TreasureContext"))
    (bind _returnvalue (`|GetDataTableRow` "/Game/Dev/Treasure/DT_TreasureContext.DT_TreasureContext" (`KismetArrayLibrary.Array_Random` _outrownames))
      (:`then`
        (return _returnvalue true))
      (:`RowNotFound`
        _)))
  (return (struct) false))

(fn `GetState`
  (returns (State :type "/Game/Dev/Chest/E_ChestState Enum"))
  (bind _state (`/Game/Dev/Chest/STM_Chest.GetState` (`self.STM_Chest`)))
  (return _state))

(fn `HideGold`
  (`SceneComponent.SetHiddenInGame` (`self.SK_Pile`) true true))

(fn `Open`
  (`/Game/Dev/Chest/STM_Chest.SendOpen` (`self.STM_Chest`)))

(fn `ShowGold`
  (`SceneComponent.SetHiddenInGame` (`self.SK_Pile`) false true))

(fn `Spawn Treasure`
  (params (Treasure :type "TreasureContext Structure"))
  (returns (`Treasure ref` :type "/Game/Dev/Treasure/BP_Treasure Object Reference"))
  (bind _outitem (`KismetArrayLibrary.Array_Random` (`|MakeArray` (`self.SocketTreasureA`) (`self.SocketTreasureB`) (`self.SocketTreasureC`))))
  (bind _returnvalue (`|SpawnActorFromClass` "/Game/Dev/Treasure/BP_Treasure.BP_Treasure_C" (`SceneComponent.GetRelativeTransform` _outitem) "Undefined" "MultiplyWithRoot" null null))
  (`self.K2_AttachToComponent` _returnvalue _outitem "None" "SnapToTarget" "SnapToTarget" "SnapToTarget" true)
  (`/Game/Dev/Treasure/BP_Treasure.Initialize` _returnvalue Treasure)
  (return _returnvalue))

(fn `UserConstructionScript`
  (`SkinnedMeshComponent.SetLeaderPoseComponent` (`self.SK_Pile`) (`self.SK_Chest`) false false))