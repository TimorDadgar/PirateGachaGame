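; Game mode for a pirate gacha game, coordinating chest openings, the gold-for-ad flow and Hector the fish's reactions.
; Chest events trigger win sounds and Hector messages, close the chest in smoke, and show non-empty loot on the shelf.
; When the pirate goes broke, input and background audio stop for an ad prompt; a finished video grants gold, while skipping just resumes play.
; A looping timer randomizes Hector's idle or flopping animation.
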(event `self.ReceiveBeginPlay`
  ;[1 1 1] Initialization
  (`KismetSystemLibrary.ExecuteConsoleCommand` "r.ScreenPercentage 100" null)
  (`KismetSystemLibrary.K2_SetTimer` null "PlayRandomFishAnimation" 5.0 true)
  (bind _returnvalue (`GameplayStatics.GetActorOfClass` "/Game/Dev/Chest/BP_Chest.BP_Chest_C"))
  (bind _output_get (set `self.Chest` _returnvalue))
  (add `/Game/Dev/Chest/BP_Chest.OnOpened` _output_get (`|CreateDelegate` :!event `OnChestOpened`))
  (add `/Game/Dev/Chest/BP_Chest.OnClosing` _output_get (`|CreateDelegate` :!event `OnChestClosing`))
  (bind _returnvalue_2 (`|CreateWidget` "/Game/UI/WBP_Ad.WBP_Ad_C"))
  (bind _output_get_2 (set `self.AdWidget` _returnvalue_2))
  (`UserWidget.AddToViewport` _output_get_2 0)
  (`Widget.SetVisibility` _returnvalue_2 "Hidden")
  (`Widget.SetVisibility` _returnvalue_2 "Hidden")
  (add `MediaPlayer.OnEndReached` (`/Game/UI/WBP_Ad.MediaPlayer` _returnvalue_2) (`|CreateDelegate` :!event `AdVideoEnd`))
  (bind _asbp_pirate (cast `/Game/Dev/Pirate/BP_Pirate` (`GameplayStatics.GetPlayerCharacter` 0)))
  (bind _output_get_3 (set `self.Pirate` _asbp_pirate))
  (add `/Game/Dev/Pirate/BP_Pirate.EventPirateBroke` _output_get_3 (`|CreateDelegate` :!event `OnPirateBroke`))
  (bind _asbp_pirate_controller (cast `/Game/Dev/Pirate/BP_PirateController` (`GameplayStatics.GetPlayerController` 0)))
  (set `self.PirateController` _asbp_pirate_controller)
  (bind _returnvalue_3 (`GameplayStatics.GetActorOfClass` "/Game/Dev/Fish/BP_Hector.BP_Hector_C"))
  (set `self.Hector` _returnvalue_3))

(event `OnPirateBroke`
  (bind _adwidget (`self.AdWidget`))
  ;[1 1 1] Pirate events
  (`/Game/Dev/Pirate/BP_PirateController.DisablePirateInput` (`self.PirateController`))
  (`Widget.SetVisibility` _adwidget "Visible")
  (`/Game/UI/WBP_Ad.HideAdVideo` _adwidget)
  (`/Game/UI/WBP_Ad.ShowAdPrompt` _adwidget)
  (bind _returnvalue (`GameplayStatics.GetActorOfClass` "/Game/Audio/background_audio_actor.background_audio_actor_C"))
  (`/Game/Audio/background_audio_actor.StopPlayingBackground` _returnvalue)
  (message `ReactionInterface.React` (`self.Hector`) "OutOfGold"))

(event `OnChestClosing`
  (params (Context :type "/Game/Dev/Chest/F_Chest Structure"))
  (bind (_luckchance _cost _loot) (break `/Game/Dev/Chest/F_Chest` Context))
  ;[1 1 1] Chest events
  (if (not (`|EnumEquality` _loot "NewEnumerator3"))
    (bind _returnvalue (`GameplayStatics.GetActorOfClass` "/Game/Dev/Shelf/BP_Shelf.BP_Shelf_C"))
    (`/Game/Dev/Shelf/BP_Shelf.ShowCollectable` _returnvalue _loot)))

(event `OnChestOpened`
  (params (Context :type "/Game/Dev/Chest/F_Chest Structure"))
  (bind _hector (`self.Hector`))
  ;[1 1 1] Chest events
  (if (`|EnumEquality` (`.Loot_29_CECEAC4D481E395414B93BAF026F0842` (break `/Game/Dev/Chest/F_Chest` Context)) "NewEnumerator3")
    (message `ReactionInterface.React` _hector "EmptyChest")
    (else
      (`self.PlayWinSound`)
      (message `ReactionInterface.React` _hector "FoundTreasure")))
  (`KismetSystemLibrary.Delay` 3.0)
  (`ActorComponent.Activate` (`/Game/Dev/Chest/BP_Chest.NS_SmokeBomb` (`self.Chest`)) true)
  (`/Game/Dev/Chest/BP_Chest.Close` (`self.Chest`)))

(event `PlayAd`
  (bind _adwidget (`self.AdWidget`))
  ;[1 1 1] Ad events
  (`/Game/UI/WBP_Ad.HideAdPrompt` _adwidget)
  (`/Game/UI/WBP_Ad.ShowAdVideo` _adwidget)
  (`/Game/UI/WBP_Ad.Play Ad Video` _adwidget))

(event `SkipAd`
  ;[1 1 1] Ad events
  (`Widget.SetVisibility` (`self.AdWidget`) "Hidden")
  (`/Game/Dev/Pirate/BP_PirateController.EnablePirateInput` (`self.PirateController`))
  (bind _returnvalue (`GameplayStatics.GetActorOfClass` "/Game/Audio/background_audio_actor.background_audio_actor_C"))
  (`/Game/Audio/background_audio_actor.StartPlayingBackground` _returnvalue))

(event `AdVideoEnd`
  ;[1 1 1] Ad events
  (bind _returnvalue (`GameplayStatics.GetActorOfClass` "/Game/Audio/background_audio_actor.background_audio_actor_C"))
  (`/Game/Audio/background_audio_actor.StartPlayingBackground` _returnvalue)
  (`Widget.SetVisibility` (`self.AdWidget`) "Hidden")
  (`/Game/Dev/Pirate/BP_Pirate.IncreasePirateGoldAndNotify` (`self.Pirate`) (`self.GoldFromAd`))
  (`/Game/Dev/Pirate/BP_PirateController.EnablePirateInput` (`self.PirateController`))
  (`self.OnGoldAdded`))

(fn `PlayRandomFishAnimation`
  (bind _outactors (`GameplayStatics.GetAllActorsOfClass` "/Game/Dev/Fish/BP_Hector.BP_Hector_C"))
  (bind _asbp_hector (cast `/Game/Dev/Fish/BP_Hector` (`|GetArrayItem` _outactors)))
  (`/Engine/EditorBlueprintResources/StandardMacros.CompareInt` (`KismetMathLibrary.RandomIntegerInRange` 1 3) 2
    (:`>`
      (if true
        (set `Hector.IsFlopping` true _asbp_hector)
        (set `Hector.IsSlowFlopping` false _asbp_hector)
        (set `Hector.IsIdle` false _asbp_hector)))
    (:`==`
      (if true
        (set `Hector.IsSlowFlopping` true _asbp_hector)
        (set `Hector.IsFlopping` false _asbp_hector)
        (set `Hector.IsIdle` false _asbp_hector)))
    (:`<`
      (if true
        (set `Hector.IsIdle` true _asbp_hector)
        (set `Hector.IsSlowFlopping` false _asbp_hector)
        (set `Hector.IsFlopping` false _asbp_hector)))))

(fn `PlayWinSound`
  (bind _audio (`self.Audio`))
  (`AudioComponent.SetSound` _audio (`KismetArrayLibrary.Array_Random` (`|MakeArray` "/Game/Audio/win/win_1-Audio.win_1-Audio" "/Game/Audio/win/win_2-Audio.win_2-Audio" "/Game/Audio/win/win_3-Audio.win_3-Audio" :!type "SoundBase Object Reference")))
  (`AudioComponent.Play` _audio 0.0))

(fn `UserConstructionScript`)