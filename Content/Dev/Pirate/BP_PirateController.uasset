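; Player controller for a mouse-driven pirate game that handles chest hovering and click interaction.
; BeginPlay shows a locked cursor and caches the player pirate and a chest reference.
; Cursor line traces set a chest's hover flag each Tick and, on left click, move and restart the pirate's Niagara marker, then pass any hit chest to the pirate.
; Custom events disable and re-enable input, and traces leave persistent debug lines.
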(event `self.ReceiveBeginPlay`
  (set `self.bShowMouseCursor` true)
  (`WidgetBlueprintLibrary.SetInputMode_GameAndUIEx` self null "LockAlways" false true)
  (bind _outactors (`GameplayStatics.GetAllActorsOfClass` "/Game/Dev/Chest/BP_Chest.BP_Chest_C"))
  (for _array_element _outactors
    (set `self.ChestRef` _array_element)
    (bind _asbp_pirate (cast `/Game/Dev/Pirate/BP_Pirate` (`GameplayStatics.GetPlayerCharacter` 0)))
    (set `self.PirateRef` _asbp_pirate)))

(event `Key|LeftMouseButton`
  (params (Key :type "Key Structure"))
  (bind (_worldlocation _worlddirection) (`self.DeprojectMousePositionToWorld`))
  (bind _ns_mouseniagara (`/Game/Dev/Pirate/BP_Pirate.NS_MouseNiagara` (`self.PirateRef`)))
  (:`Pressed`
    (bind _outhit (`KismetSystemLibrary.LineTraceSingle` :`Start` _worldlocation :`End` (+ _worldlocation (* _worlddirection 10000.0)) :`TraceChannel` "TraceTypeQuery1" :`DrawDebugType` "Persistent"))
    (bind (_bblockinghit _binitialoverlap _time _distance _location _impactpoint _normal _impactnormal _physmat _hitactor) (`GameplayStatics.BreakHitResult` _outhit))
    (`SceneComponent.K2_SetWorldLocation` _ns_mouseniagara _location false false)
    (`KismetSystemLibrary.Delay` 0.1)
    (`NiagaraComponent.ResetSystem` _ns_mouseniagara)
    (`KismetSystemLibrary.PrintString` "Spawn Niagara")
    (bind _asbp_chest (cast `/Game/Dev/Chest/BP_Chest` _hitactor))
    (`/Game/Dev/Pirate/BP_Pirate.InteractWithChest` (`self.PirateRef`) _asbp_chest)))

(event `DisablePirateInput`
  (`self.DisableInput` null))

(event `EnablePirateInput`
  (`self.EnableInput` null))

(event `self.ReceiveTick`
  (params (DeltaSeconds :type "Float (single-precision)"))
  (bind (_worldlocation _worlddirection) (`self.DeprojectMousePositionToWorld`))
  (bind _outhit (`KismetSystemLibrary.LineTraceSingle` :`Start` _worldlocation :`End` (+ _worldlocation (* _worlddirection 10000.0)) :`TraceChannel` "TraceTypeQuery1" :`DrawDebugType` "Persistent"))
  (bind _asbp_chest (cast `/Game/Dev/Chest/BP_Chest` (`.HitActor` (`GameplayStatics.BreakHitResult` _outhit)))
    (:`then`
      (bind _output_get (set `self.ChestRef` _asbp_chest))
      (set `Chest.IsHovering` true _output_get)
      (`KismetSystemLibrary.PrintString` "Hovering"))
    (:`CastFailed`
      (set `Chest.IsHovering` false (`self.ChestRef`)))))

(fn `UserConstructionScript`)