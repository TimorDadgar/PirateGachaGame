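; BP_Pirate is a pirate that holds a gold balance and spends it to open chests.
; InteractWithChest gets the chest's cost, then either deducts the gold and opens the chest, or prints a message and raises a pirate-broke event.
; Helpers that increase or decrease the gold raise a gold-changed event, which also fires on BeginPlay to broadcast the starting amount.
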(event `self.ReceiveBeginPlay`
  (`self.EventPirateGoldChanged` (`self.PirateGold`)))

(fn `CanAfford`
  (params (Cost :type Integer))
  (returns (canAfford :type Boolean))
  (return (>= (`self.PirateGold`) Cost)))

(fn `DecreasePirateGoldAndNotify`
  (params (GoldToDecrease :type Integer))
  (bind _output_get (set `self.PirateGold` (- (`self.PirateGold`) GoldToDecrease)))
  (`self.EventPirateGoldChanged` _output_get))

(fn `IncreasePirateGoldAndNotify`
  (params (GoldToIncrease :type Integer))
  (bind _output_get (set `self.PirateGold` (+ (`self.PirateGold`) GoldToIncrease)))
  (`self.EventPirateGoldChanged` _output_get))

(fn `InteractWithChest`
  (params (Chest :type "/Game/Dev/Chest/BP_Chest Object Reference"))
  (bind _cost (`/Game/Dev/Chest/BP_Chest.GetCost` Chest))
  (bind _canafford (`self.CanAfford` _cost))
  (if _canafford
    (`self.DecreasePirateGoldAndNotify` _cost)
    (`/Game/Dev/Chest/BP_Chest.OpenChest` Chest)
    (else
      (`KismetSystemLibrary.PrintString` "I can't afford... :(")
      (`self.EventPirateBroke`))))

(fn `UserConstructionScript`)