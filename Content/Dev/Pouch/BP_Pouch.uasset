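; BP_Pouch is the gold pouch actor that displays the pirate's gold total and reacts to gold earned from ads.
; On BeginPlay it binds to the game mode's gold-added-from-ad dispatcher and to the gold-changed dispatcher on the BP_Pirate found in the level.
; Gold changes update the world-space coin text.
; Ad rewards activate the coin Niagara effect and play a random pickup sound.
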(event `self.ReceiveBeginPlay`
  (bind _asbp_pirate_gacha_game_mode (cast `/Game/Dev/Mode/BP_PirateGachaGameMode` (`GameplayStatics.GetGameMode`)))
  (add `/Game/Dev/Mode/BP_PirateGachaGameMode.ED_GoldAddedFromAd` _asbp_pirate_gacha_game_mode (delegate `GoldAdded`))
  (bind _returnvalue (`GameplayStatics.GetActorOfClass` "/Game/Dev/Pirate/BP_Pirate.BP_Pirate_C"))
  (add `/Game/Dev/Pirate/BP_Pirate.EventPirateGoldChanged` _returnvalue (delegate `GoldChanged`)))

(event `GoldAdded`
  (bind _audio (`self.Audio`))
  (`ActorComponent.Activate` (`self.NS_Coins`) true)
  (`AudioComponent.SetSound` _audio (`KismetArrayLibrary.Array_Random` (`|MakeArray` "/Game/Audio/kaching/getGold_1-Audio.getGold_1-Audio" "/Game/Audio/kaching/getGold_2-Audio.getGold_2-Audio" "/Game/Audio/kaching/getGold_3-Audio.getGold_3-Audio" "/Game/Audio/kaching/getGold_4-Audio.getGold_4-Audio" "/Game/Audio/kaching/getGold_5-Audio.getGold_5-Audio" :!type "SoundBase Object Reference")))
  (`AudioComponent.Play` _audio 0.0))

(event `GoldChanged`
  (params (NewGoldAmount :type Integer))
  (`TextRenderComponent.K2_SetText` (`self.CoinWorldText`) (`KismetTextLibrary.Conv_IntToText` NewGoldAmount)))

(fn `UserConstructionScript`)